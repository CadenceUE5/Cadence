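; BP_GestureRecorder is an actor that draws gestures on a plane, exports them to a JSON database and matches player gestures against stored ones.
; Construction binds a render target (shared for target gestures, otherwise created) to the plane's material and builds the database path under game source.
; GestureBrush stamps a brush material at normalized canvas positions.
; Export appends auto-named point lists, while CompareToTargetGestures returns the first successful match, logging distance and direction errors.
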(event EventBeginPlay)

(event Collision|EventActorBeginOverlap
  (params (OtherActor :type Actor%20Object%20Reference)))

(event EventTick
  (params (DeltaSeconds :type Float%20%28single-precision%29)))

(fn ConstructionScript
  (Utilities|FlowControl|Sequence
    (:then_0
      (if (Variables|Default|GetbIsTargetGesture)
        (Variables|Default|SetRender%20Target "/Game/Gesture/RT_TargetGesture.RT_TargetGesture")
        (else
          (bind _returnvalue (Rendering|CreateRenderTarget2D 1024 1024 "RTF_RGBA16f" "(R=1.000000,G=1.000000,B=1.000000,A=1.000000)" false true))
          (Variables|Default|SetRender%20Target _returnvalue))))
    (:then_1
      (bind _returnvalue_2 (Rendering|Material|CreateDynamicMaterialInstance (Rendering|Material|GetMaterial (Variables|Default|GetPlane) 0) "None" "None" :!class /Script/Engine.KismetMaterialLibrary))
      (Rendering|Material|SetTextureParameterValue _returnvalue_2 "Texture" (Variables|Default|GetRender%20Target))
      (Rendering|Material|SetMaterial (Variables|Default|GetPlane) 0 _returnvalue_2))
    (:then_2
      (bind _returnvalue_3 (Rendering|Material|CreateDynamicMaterialInstance "/Game/Gesture/M_GestureFG.M_GestureFG" "None" "None" :!class /Script/Engine.KismetMaterialLibrary))
      (Variables|Default|SetBrush _returnvalue_3))
    (:then_3
      (Variables|Default|Setm_DatabaseFilePath (Utilities|String|Append (Class|BlueprintPathsLibrary|GameSourceDir) "Cadence/Gesture/Exports/" (Variables|Default|GetGesturePrefix) "GestureData.json")))))

(fn GestureBrush
  (params (Size :type Float%20%28double-precision%29) (Location :type Vector%202D%20Structure))
  (bind _returnvalue (/ Size 2.0))
  (bind (_canvas _size _context) (Rendering|BeginDrawCanvastoRenderTarget (Variables|Default|GetRender%20Target)))
  (Canvas|DrawMaterial :self _canvas :RenderMaterial (Variables|Default|GetBrush) :ScreenPosition (- (* _size Location) (Math|Vector2D|MakeVector2D _returnvalue _returnvalue)) :ScreenSize (Math|Vector2D|MakeVector2D Size Size) :CoordinateSize "(X=1.000000,Y=1.000000)" :PivotPoint "(X=0.500000,Y=0.500000)")
  (Rendering|EndDrawCanvastoRenderTarget _context))

(fn Export
  (params (Points :type Array%20of%20Vector%202D%20Structures))
  (bind _returnvalue (Class|AGestureRecorder|GetGestureCount))
  (Class|AGestureRecorder|AppendGesturetoDatabase (Variables|Default|Getm_DatabaseFilePath) (Utilities|Struct|MakeGestureData (Utilities|String|Append (Variables|Default|GetGesturePrefix) (Utilities|String|ToString(Integer) _returnvalue)) Points))
  (if true
    (Development|PrintString "BPGestureRecorder - Data table exported successfully.")
    (Utilities|Array|Clear Points)))

(fn ComparetoTargetGestures
  (params (Player%20Points :type Array%20of%20Vector%202D%20Structures))
  (bind _returnvalue (Class|AGestureRecorder|GetAllGestures))
  (for _array_element _returnvalue
    (Development|PrintString (Utilities|String|Append "BPGestureRecorder - Comparing player gesture to " (.GestureName (Utilities|Struct|BreakGestureData _array_element))))
    (bind (_successbool _distanceerror _directionerror) (CallFunction|MatchGesture Player%20Points (.Points (Utilities|Struct|BreakGestureData _array_element))))
    (Development|PrintString (Utilities|String|Append "BPGestureRecorder - Distance Error: " (Utilities|String|ToString(Float) _distanceerror) ", Direction Error: " (Utilities|String|ToString(Float) _directionerror)))
    (if _successbool
      (Development|PrintString (Utilities|String|Append "BPGestureRecorder - Matched successfully with " (.GestureName (Utilities|Struct|BreakGestureData _array_element)) "!"))
      (return true _array_element)))
  (Development|PrintString "BPGestureRecorder - No match found.")
  (return false ""))