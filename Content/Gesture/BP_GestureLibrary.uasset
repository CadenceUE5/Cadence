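; Gesture library that compares a player's 2D point stroke against a reference gesture.
; MatchGesture centres both strokes on their bounding boxes and scales them by the longer side.
; It then averages index-paired point distance and angle between segment directions, without resampling, so only the shorter length is compared.
; As written, it returns true when both errors exceed their thresholds, not when they fall below.
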(fn NormalizePoints
  (params (PointArray :type Array%20of%20Vector%202D%20Structures))
  (for _array_element PointArray
    ;[0.15 0.15 0.15 0.5] setting min max vals
    (if (> (.X (Math|Vector2D|BreakVector2D _array_element)) (LocalVariables|GetMaxX))
      (LocalVariables|SetMaxX (.X (Math|Vector2D|BreakVector2D _array_element))))
    (if (< (.X (Math|Vector2D|BreakVector2D _array_element)) (LocalVariables|GetMinX))
      (LocalVariables|SetMinX (.X (Math|Vector2D|BreakVector2D _array_element))))
    (if (> (.Y (Math|Vector2D|BreakVector2D _array_element)) (LocalVariables|GetMaxY))
      (LocalVariables|SetMaxY (.Y (Math|Vector2D|BreakVector2D _array_element))))
    (if (< (.Y (Math|Vector2D|BreakVector2D _array_element)) (LocalVariables|GetMinY))
      (LocalVariables|SetMinY (.Y (Math|Vector2D|BreakVector2D _array_element)))))
  (for _array_element_2 PointArray
    (Utilities|Array|Add (LocalVariables|GetNormPoints) (/ (- _array_element_2 (Math|Vector2D|MakeVector2D (+ (LocalVariables|GetMinX) (* (- (LocalVariables|GetMaxX) (LocalVariables|GetMinX)) 0.5)) (+ (* (- (LocalVariables|GetMaxY) (LocalVariables|GetMinY)) 0.5) (LocalVariables|GetMinY)))) (Math|Float|Max(Float) (- (LocalVariables|GetMaxX) (LocalVariables|GetMinX)) (- (LocalVariables|GetMaxY) (LocalVariables|GetMinY))))))
  (return (LocalVariables|GetNormPoints)))

(fn MatchGesture
  (params (PlayerPoints :type Array%20of%20Vector%202D%20Structures) (ReferencePoints :type Array%20of%20Vector%202D%20Structures))
  (bind _normalizedpoints (CallFunction|NormalizePoints PlayerPoints))
  (bind _normalizedpoints_2 (CallFunction|NormalizePoints ReferencePoints))
  (bind _errorvalue (CallFunction|CalculateDistanceError _normalizedpoints _normalizedpoints_2))
  (bind _directionerror (CallFunction|CalcuateDirectionError _normalizedpoints _normalizedpoints_2))
  (return (and (< (LocalVariables|GetDistanceThreshold) _errorvalue) (< (LocalVariables|GetDirectionThreshold) _directionerror))))

(fn CalcuateDirectionError
  (params (PlayerPoints :type Array%20of%20Vector%202D%20Structures) (ReferencePoints :type Array%20of%20Vector%202D%20Structures))
  (bind _playerdirs (LocalVariables|GetPlayerDirs))
  (bind _referencedirs (LocalVariables|GetReferenceDirs))
  (bind _returnvalue (Utilities|Array|Length _playerdirs))
  (bind _returnvalue_2 (Utilities|Array|Length _referencedirs))
  (bind _returnvalue_3 (Math|Integer|Min(Integer) _returnvalue _returnvalue_2))
  ;[0.15 0.15 0.15 0.5] player dir vectors
  (for _index (range 0 (- (Utilities|Array|Length PlayerPoints) 2))
    (Utilities|Array|Add (LocalVariables|GetPlayerDirs) (Math|Vector2D|Normalize2D (- (Utilities|Array|Get(acopy) PlayerPoints (+ _index 1)) (Utilities|Array|Get(acopy) PlayerPoints _index)))))
  ;[0.15 0.15 0.15 0.5] reference dir vectors
  (for _index_2 (range 0 (- (Utilities|Array|Length ReferencePoints) 2))
    (Utilities|Array|Add (LocalVariables|GetReferenceDirs) (Math|Vector2D|Normalize2D (- (Utilities|Array|Get(acopy) ReferencePoints (+ _index_2 1)) (Utilities|Array|Get(acopy) ReferencePoints _index_2)))))
  (for _index_3 (range 0 (- _returnvalue_3 1))
    ;[0.15 0.15 0.15 0.5] accumulate error
    (LocalVariables|SetAccumError (+ (LocalVariables|GetAccumError) (Math|Trig|Acos(Degrees) (Math|Vector2D|DotProduct(2D) (Utilities|Array|Get(acopy) (LocalVariables|GetPlayerDirs) _index_3) (Utilities|Array|Get(acopy) (LocalVariables|GetReferenceDirs) _index_3))))))
  (return (/ (LocalVariables|GetAccumError) _returnvalue_3)))

(fn CalculateDistanceError
  (params (PlayerPoints :type Array%20of%20Vector%202D%20Structures) (ReferencePoints :type Array%20of%20Vector%202D%20Structures))
  (bind _returnvalue (Utilities|Array|Length PlayerPoints))
  (bind _returnvalue_2 (Utilities|Array|Length ReferencePoints))
  (bind _returnvalue_3 (Math|Integer|Min(Integer) _returnvalue _returnvalue_2))
  (for _index (range 0 (- _returnvalue_3 1))
    (LocalVariables|SetAccumulatedError (+ (LocalVariables|GetAccumulatedError) (Math|Vector|Distance2D(Vector) (Utilities|Array|Get(acopy) PlayerPoints _index) (Utilities|Array|Get(acopy) ReferencePoints _index)))))
  (return (/ (LocalVariables|GetAccumulatedError) _returnvalue_3)))