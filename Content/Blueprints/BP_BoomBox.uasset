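; BP_BoomBox is a boombox actor that checks the looper against a goal sound when something overlaps its first button collider.
; On overlap it uses its LooperRef, fetching LooperMaster from the GI_Cadence game instance if the reference is invalid.
; It passes LoadedGoalSound's class defaults to the looper's exact and tolerance-based validations, then only prints both results as debug strings.
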(event OnComponentBeginOverlap(ColliderButton1)
  (params (OverlappedComponent :type Primitive%20Component%20Object%20Reference) (OtherActor :type Actor%20Object%20Reference) (OtherComp :type Primitive%20Component%20Object%20Reference) (OtherBodyIndex :type Integer) (bFromSweep :type Boolean) (SweepResult :type Hit%20Result%20Structure%20%28by%20ref%29))
  (bind _matchtolerance (Variables|Default|GetMatchTolerance))
  (bind _loadedgoalsound (Variables|Default|GetLoadedGoalSound))
  (bind _time_to_sound_map (Utilities|GetClassDefaults _loadedgoalsound))
  (Variables|Default|GetLooperRef
    (:then
      _)
    (:else
      (bind _asgi_cadence (Utilities|Casting|CastToGI_Cadence (Game|GetGameInstance)))
      (Variables|Default|SetLooperRef (Variables|/Game/Performance/GI_Cadence.GI_Cadence_C|GetLooperMaster _asgi_cadence))))
  (Utilities|FlowControl|Sequence
    (:then_0
      (bind _comparison_result (Default|ValidateExact (Variables|Default|GetLooperRef) _time_to_sound_map))
      (Development|PrintString (Utilities|String|Append "BPBoomBox - Validate Exact Match Result: " (Utilities|String|ToString(Boolean) _comparison_result))))
    (:then_1
      (bind _maps_equivalent (Default|ValidateTolerance (Variables|Default|GetLooperRef) _time_to_sound_map _matchtolerance))
      (Development|PrintString (Utilities|String|Append "BPBoomBox - Validate Match with Tolerance of " (Utilities|String|ToString(Float) _matchtolerance) " Result: " (Utilities|String|ToString(Boolean) _maps_equivalent))))))

(event EventBeginPlay)

(event Collision|EventActorBeginOverlap
  (params (OtherActor :type Actor%20Object%20Reference)))

(event EventTick
  (params (DeltaSeconds :type Float%20%28single-precision%29)))

(fn ConstructionScript)