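; BP_LooperV2 is a timer-driven audio looper that plays 2D sounds stored in a map keyed by time within the loop.
; A repeating LoopLength timer runs PerformLoop, which starts a new looping DoBeat timer each call, fires beat and loop dispatchers, and advances the beat counter.
; DoBeat plays sounds matching the beat-rounded time.
; AddSound files new sounds under the current rounded time; BeginPlay seeds demo sounds.
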(event Custom|Perform%20Loop
  (Utilities|Time|SetTimerbyEvent (delegate Custom|Do%20Beat) (stale EventBeginPlay _output_get) true)
  (CallFunction|DoBeat)
  (Default|CallEDDispatchBeat (Variables|Default|GetBeats%20Completed))
  (if (== (Variables|Default|GetBeats%20Completed) 0)
    (Default|CallEDDispatchLoop))
  (Math|Integer|IncrementInt (Variables|Default|GetBeats%20Completed)
    (:%20%20
      (if (>= (Variables|Default|GetBeats%20Completed) (* (Variables|Default|GetBeats%20per%20Bar) (Variables|Default|GetBars%20per%20Loop)))
        (Development|PrintString "Loop Complete")
        (Variables|Default|SetBeats%20Completed 0)))))

(event Custom|Do%20Beat
  (bind _times_to_sound_map (Variables|Default|GetTimes%20to%20Sound%20Map))
  (bind _loop_timer_handle (Variables|Default|GetLoop%20Timer%20Handle))
  (bind _beats_per_bar (Variables|Default|GetBeats%20per%20Bar))
  (bind _beats_completed (Variables|Default|GetBeats%20Completed))
  (bind _time_per_beat (Variables|Default|GetTime%20per%20Beat))
  (bind _returnvalue (Class|KismetSystemLibrary|GetTimerElapsedTimeHandle _loop_timer_handle))
  (bind _returnvalue_2 (* _beats_completed _time_per_beat))
  (bind _returnvalue_3 (* _returnvalue _beats_per_bar))
  (bind _rounded_time (CallFunction|RoundTimetoNearestBeat _returnvalue_3 _beats_per_bar))
  (bind _returnvalue_4 (+ _rounded_time _returnvalue_2))
  (bind (_value _returnvalue_5) (Utilities|Map|Find _times_to_sound_map _returnvalue_4))
  (if _returnvalue_5
    (for _array_element (Utilities|Struct|BreakS_AudioMapData _value)
      (Audio|PlaySound2D _array_element 1.0 1.0 0.0 0 0))))

(event EventBeginPlay
  (bind _output_get (Variables|Default|SetTime%20per%20Beat (Utilities|Operators|Divide (Variables|Default|GetLoop%20Length) (Variables|Default|GetBars%20per%20Loop) (Variables|Default|GetBeats%20per%20Bar))))
  (bind _returnvalue (Utilities|Time|SetTimerbyEvent (delegate Custom|Perform%20Loop) (Variables|Default|GetLoop%20Length) true))
  (Variables|Default|SetLoop%20Timer%20Handle _returnvalue)
  (CallFunction|SetupDemoSounds))

(fn ConstructionScript)

(fn SetupDemoSounds
  (bind _array (Utilities|Array|MakeArray "/Engine/EngineSounds/1kSineTonePing.1kSineTonePing" "/Engine/VREditor/Sounds/UI/Click_on_Button_Cue.Click_on_Button_Cue"))
  (bind _times_to_sound_map (Variables|Default|GetTimes%20to%20Sound%20Map))
  (bind _s_audiomapdata (Utilities|Struct|MakeS_AudioMapData _array))
  (Utilities|Map|Add _times_to_sound_map 0.25 (Utilities|Struct|MakeS_AudioMapData (Utilities|Array|MakeArray "/Engine/EngineSounds/1kSineTonePing.1kSineTonePing" "/Engine/VREditor/Sounds/UI/Camera_Shutter.Camera_Shutter")))
  (Utilities|Map|Add _times_to_sound_map 0.5 _s_audiomapdata)
  (Utilities|Map|Add _times_to_sound_map 1.0 _s_audiomapdata))

(fn AddSound
  (params (Sound%20to%20Add :type Sound%20Base%20Object%20Reference))
  (bind _times_to_sound_map (Variables|Default|GetTimes%20to%20Sound%20Map))
  (bind _output_get (LocalVariables|SetCurrent%20Time%20in%20Overall%20Loop (CallFunction|RoundTimetoNearestBeat (+ (* (Variables|Default|GetBeats%20Completed) (Variables|Default|GetTime%20per%20Beat)) (Class|KismetSystemLibrary|GetTimerElapsedTimeHandle (Variables|Default|GetLoop%20Timer%20Handle))) (Variables|Default|GetBeats%20per%20Bar))))
  (Utilities|FlowControl|Sequence
    (:then_0
      (if (.ReturnValue (Utilities|Map|Find _times_to_sound_map _output_get))
        (Utilities|Array|Add (Utilities|Struct|BreakS_AudioMapData (.Value (Utilities|Map|Find _times_to_sound_map _output_get))) Sound%20to%20Add)
        (else
          (Utilities|Map|Add _times_to_sound_map _output_get (Utilities|Struct|MakeS_AudioMapData (Utilities|Array|MakeArray Sound%20to%20Add))))))
    (:then_1
      (Development|PrintString (Utilities|String|ToString(Float) _output_get)))))