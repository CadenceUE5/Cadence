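; BP_Looper_User is an audio looper Blueprint that records sounds added during playback into a timed loop.
; AddSound timestamps each sound from the loop timer, optionally snapped to the nearest beat, groups it in a time-to-sounds map and fires a dispatcher.
; RemoveSound drops the last sound stored at MostRecentTime.
; BeginPlay defers to the parent, and an unconnected test event adds sample sounds after short delays.
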(event Custom|Test%20Sound%20Add
  (Utilities|FlowControl|Delay 0.5)
  (CallFunction|AddSound "/Game/Audio/sound_effect/trash/beer-can.beer-can")
  (Utilities|FlowControl|Delay 0.5)
  (CallFunction|AddSound "/Game/Audio/sound_effect/trash/can-thrown.can-thrown")
  (Utilities|FlowControl|Delay 0.66)
  (CallFunction|AddSound "/Engine/EditorSounds/Notifications/CompileFailed.CompileFailed"))

(event EventBeginPlay
  (|CallParentFunction))

(event Collision|EventActorBeginOverlap
  (params (OtherActor :type Actor%20Object%20Reference)))

(event EventTick
  (params (DeltaSeconds :type Float%20%28single-precision%29)))

(fn ConstructionScript
  (|CallParentFunction))

(fn AddSound
  (params (Sound%20to%20Add :type Sound%20Base%20Object%20Reference))
  (bind _times_to_sound_map (Variables|Default|GetTimes%20to%20Sound%20Map))
  (bind _loop_timer_handle (Variables|Default|GetLoop%20Timer%20Handle))
  (bind _returnvalue (Class|KismetSystemLibrary|GetTimerElapsedTimeHandle _loop_timer_handle))
  (Utilities|FlowControl|Sequence
    (:then_0
      (if (Variables|Default|GetLock%20Added%20Sounds%20to%20Beat)
        (LocalVariables|SetCurrent%20Time%20in%20Overall%20Loop (CallFunction|RoundTimetoNearestBeat (+ (* (Variables|Default|GetBeats%20Completed) (Variables|Default|GetTime%20per%20Beat)) _returnvalue) (/ (Variables|Default|GetLoop%20Length) (Variables|Default|GetBars%20per%20Loop)) (Variables|Default|GetBeats%20per%20Bar)))
        (else
          (LocalVariables|SetCurrent%20Time%20in%20Overall%20Loop _returnvalue))))
    (:then_1
      (if (.ReturnValue (Utilities|Map|Find _times_to_sound_map (LocalVariables|GetCurrent%20Time%20in%20Overall%20Loop)))
        (Utilities|Array|Add (Utilities|Struct|BreakS_AudioMapData (.Value (Utilities|Map|Find _times_to_sound_map (LocalVariables|GetCurrent%20Time%20in%20Overall%20Loop)))) Sound%20to%20Add)
        (else
          (Utilities|Map|Add _times_to_sound_map (LocalVariables|GetCurrent%20Time%20in%20Overall%20Loop) (Utilities|Struct|MakeS_AudioMapData (Utilities|Array|MakeArray Sound%20to%20Add))))))
    (:then_2
      (Default|CallEDDispatchSoundAdded))))

(fn RemoveSound
  (bind _times_to_sound_map (Variables|Default|GetTimes%20to%20Sound%20Map))
  (bind _most_recent_time (Variables|Default|GetMost%20Recent%20Time))
  (bind (_value _returnvalue) (Utilities|Map|Find _times_to_sound_map _most_recent_time))
  (bind _soundsarray (Utilities|Struct|BreakS_AudioMapData _value))
  (if _returnvalue
    (Utilities|Array|RemoveIndex _soundsarray (- (Utilities|Array|Length _soundsarray) 1))))