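; BP_LooperAmy is an audio looper that replays a time-to-sounds map every loop and broadcasts loop and beat events.
; BeginPlay applies an optional preset and starts a looping timer, which restarts the beat timer and chains delays through the sorted times to play 2D sounds.
; AddSound records at the current loop time, optionally beat-snapped.
; Validate functions compare the map to another, exactly or within a time tolerance.
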(event Custom|Perform%20Loop
  (Utilities|Time|SetTimerbyEvent (delegate Custom|Do%20Beat) (stale EventBeginPlay _output_get) true)
  (Default|CallEDDispatchLoop)
  (Variables|Default|SetBeats%20Completed 0)
  (CallFunction|PlayLoopSounds))

(event Custom|Do%20Beat
  (Default|CallEDDispatchBeat (Variables|Default|GetBeats%20Completed))
  (Math|Integer|IncrementInt (Variables|Default|GetBeats%20Completed)))

(event Custom|Play%20Loop%20Sounds
  (bind _times_to_sound_map (Variables|Default|GetTimes%20to%20Sound%20Map))
  (bind _keys (Utilities|Map|Keys _times_to_sound_map))
  (bind _output_get (Variables|Default|SetTimes%20of%20Sounds _keys))
  (Class|KismetArrayLibrary|SortFloatArray _output_get)
  (Utilities|FlowControl|Delay (Utilities|Array|Get(acopy) (Variables|Default|GetTimes%20of%20Sounds)))
  (for _array_element (Utilities|Struct|BreakS_AudioMapData (.Value (Utilities|Map|Find _times_to_sound_map (Utilities|Array|Get(acopy) (Variables|Default|GetTimes%20of%20Sounds)))))
    (Audio|PlaySound2D _array_element 1.0 1.0 0.0 0 0))
  (if (> (Utilities|Map|Length (Variables|Default|GetTimes%20to%20Sound%20Map)) 1)
    (CallFunction|PlayNextSound 1)))

(event Custom|Play%20Next%20Sound
  (params (Index :type Integer))
  (bind _times_of_sounds (Variables|Default|GetTimes%20of%20Sounds))
  (bind _output (Utilities|Array|Get(acopy) _times_of_sounds Index))
  (Utilities|FlowControl|Delay (- _output (Utilities|Array|Get(acopy) _times_of_sounds (- Index 1))))
  (for _array_element (Utilities|Struct|BreakS_AudioMapData (.Value (Utilities|Map|Find (Variables|Default|GetTimes%20to%20Sound%20Map) _output)))
    (Audio|PlaySound2D _array_element 1.0 1.0 0.0 0 0))
  (if (> (- (Utilities|Array|Length (Variables|Default|GetTimes%20of%20Sounds)) Index) 1)
    (CallFunction|PlayNextSound (+ Index 1))))

(event EventBeginPlay
  (CallFunction|CheckforPreset)
  (bind _output_get (Variables|Default|SetTime%20per%20Beat (Utilities|Operators|Divide (Variables|Default|GetLoop%20Length) (Variables|Default|GetBars%20per%20Loop) (Variables|Default|GetBeats%20per%20Bar))))
  (bind _returnvalue (Utilities|Time|SetTimerbyEvent (delegate Custom|Perform%20Loop) (Variables|Default|GetLoop%20Length) true))
  (Variables|Default|SetLoop%20Timer%20Handle _returnvalue)
  (if (Utilities|Map|IsEmpty (Variables|Default|GetTimes%20to%20Sound%20Map))
    _))

(fn ConstructionScript)

(fn SetupDemoSounds
  (bind _array (Utilities|Array|MakeArray "/Engine/EngineSounds/1kSineTonePing.1kSineTonePing" "/Engine/VREditor/Sounds/UI/Click_on_Button_Cue.Click_on_Button_Cue"))
  (bind _array_2 (Utilities|Array|MakeArray "/Engine/EngineSounds/1kSineTonePing.1kSineTonePing" "/Engine/VREditor/Sounds/UI/Camera_Shutter.Camera_Shutter"))
  (bind _times_to_sound_map (Variables|Default|GetTimes%20to%20Sound%20Map))
  (bind _s_audiomapdata (Utilities|Struct|MakeS_AudioMapData _array))
  (bind _s_audiomapdata_2 (Utilities|Struct|MakeS_AudioMapData _array_2))
  (Variables|Default|SetLoop%20Length 4.0)
  (Utilities|Map|Add _times_to_sound_map 0.25 _s_audiomapdata_2)
  (Utilities|Map|Add _times_to_sound_map 0.5 _s_audiomapdata)
  (Utilities|Map|Add _times_to_sound_map 1.0 _s_audiomapdata)
  (Utilities|Map|Add _times_to_sound_map 1.66 _s_audiomapdata_2))

(fn AddSound
  (params (Sound%20to%20Add :type Sound%20Base%20Object%20Reference))
  (bind _times_to_sound_map (Variables|Default|GetTimes%20to%20Sound%20Map))
  (bind _loop_timer_handle (Variables|Default|GetLoop%20Timer%20Handle))
  (bind _returnvalue (Class|KismetSystemLibrary|GetTimerElapsedTimeHandle _loop_timer_handle))
  (Utilities|FlowControl|Sequence
    (:then_0
      (if (Variables|Default|GetLock%20Added%20Sounds%20to%20Beat)
        (LocalVariables|SetCurrent%20Time%20in%20Overall%20Loop (CallFunction|RoundTimetoNearestBeat (+ (* (Variables|Default|GetBeats%20Completed) (Variables|Default|GetTime%20per%20Beat)) _returnvalue) (/ (Variables|Default|GetLoop%20Length) (Variables|Default|GetBars%20per%20Loop)) (Variables|Default|GetBeats%20per%20Bar)))
        (else
          (LocalVariables|SetCurrent%20Time%20in%20Overall%20Loop _returnvalue))))
    (:then_1
      (if (.ReturnValue (Utilities|Map|Find _times_to_sound_map (LocalVariables|GetCurrent%20Time%20in%20Overall%20Loop)))
        (Utilities|Array|Add (Utilities|Struct|BreakS_AudioMapData (.Value (Utilities|Map|Find _times_to_sound_map (LocalVariables|GetCurrent%20Time%20in%20Overall%20Loop)))) Sound%20to%20Add)
        (else
          (Utilities|Map|Add _times_to_sound_map (LocalVariables|GetCurrent%20Time%20in%20Overall%20Loop) (Utilities|Struct|MakeS_AudioMapData (Utilities|Array|MakeArray Sound%20to%20Add))))))))

(fn CheckforPreset
  (bind _looper_settings_preset (Variables|Default|GetLooper%20Settings%20Preset))
  (bind _psoundmap (Variables|/Game/Audio/Blueprints/BP_LooperSettingsPreset.BP_LooperSettingsPreset_C|GetPSoundMap _looper_settings_preset))
  (bind _plooplength (Variables|/Game/Audio/Blueprints/BP_LooperSettingsPreset.BP_LooperSettingsPreset_C|GetPLoopLength _looper_settings_preset))
  (Utilities|IsValid _looper_settings_preset
    (:Is%20Valid
      (Utilities|FlowControl|Sequence
        (:then_0
          (if (Utilities|Map|IsNotEmpty _psoundmap)
            (Variables|Default|SetTimes%20to%20Sound%20Map _psoundmap)))
        (:then_1
          (if (> _plooplength 0.0)
            (Variables|Default|SetLoop%20Length _plooplength)))))))

(fn ValidateExact
  (params (Map%20to%20Compare%20Against :type Map%20of%20Floats%20%28double-precision%29%20to%20Structs))
  (LocalVariables|SetMaps%20Equal (== (Utilities|Map|Length Map%20to%20Compare%20Against) (Utilities|Map|Length (Variables|Default|GetTimes%20to%20Sound%20Map))))
  (bind (_keypin _valuepin) (Utilities|Map|ForEachLoop(Map) Map%20to%20Compare%20Against)
    (:then
      (if (.ReturnValue (Utilities|Map|Find (Variables|Default|GetTimes%20to%20Sound%20Map) _keypin))
        (if (== (Utilities|Array|Length (Utilities|Struct|BreakS_AudioMapData (.Value (Utilities|Map|Find (Variables|Default|GetTimes%20to%20Sound%20Map) _keypin)))) (Utilities|Array|Length (Utilities|Struct|BreakS_AudioMapData _valuepin)))
          (for (_array_element _array_index) (Utilities|Struct|BreakS_AudioMapData (.Value (Utilities|Map|Find (Variables|Default|GetTimes%20to%20Sound%20Map) _keypin)))
            (LocalVariables|SetMaps%20Equal (or (LocalVariables|GetMaps%20Equal) (== _array_element (Utilities|Array|Get(acopy) (Utilities|Struct|BreakS_AudioMapData _valuepin) _array_index)))))
          (else
            (LocalVariables|SetMaps%20Equal false)))
        (else
          (LocalVariables|SetMaps%20Equal false))))
    (:CompletedPin
      (return (LocalVariables|GetMaps%20Equal)))))

(fn ValidateTolerance
  (params (Map%20to%20Compare%20Against :type Map%20of%20Floats%20%28double-precision%29%20to%20Structs) (Tolerance :type Float%20%28double-precision%29))
  (bind _times_to_sound_map (Variables|Default|GetTimes%20to%20Sound%20Map))
  (bind _returnvalue (Utilities|Map|Length _times_to_sound_map))
  (bind _output_get (LocalVariables|SetReturn (== (Utilities|Map|Length Map%20to%20Compare%20Against) _returnvalue)))
  (if _output_get
    (bind _keys (Utilities|Map|Keys (Variables|Default|GetTimes%20to%20Sound%20Map)))
    (bind _keys_2 (Utilities|Map|Keys Map%20to%20Compare%20Against))
    (for _array_element _keys
      (bind _array_element_2 (Utilities|Array|ForEachLoopwithBreak _keys_2 :!label _label)
        (:LoopBody
          (if (<= (Math|Float|Absolute(Float) (- _array_element _array_element_2)) Tolerance)
            (Utilities|Map|Add (LocalVariables|GetLocal%20to%20Matched%20Time%20Map) _array_element _array_element_2)
            (goto _label Break)))))
    (if (== (Utilities|Map|Length (LocalVariables|GetLocal%20to%20Matched%20Time%20Map)) _returnvalue)
      (bind (_keypin _valuepin) (Utilities|Map|ForEachLoop(Map) (LocalVariables|GetLocal%20to%20Matched%20Time%20Map))
        (:then
          (if (== (Utilities|Array|Length (Utilities|Struct|BreakS_AudioMapData (.Value (Utilities|Map|Find (Variables|Default|GetTimes%20to%20Sound%20Map) _keypin)))) (Utilities|Array|Length (Utilities|Struct|BreakS_AudioMapData (.Value (Utilities|Map|Find Map%20to%20Compare%20Against _valuepin)))))
            (for _array_element_3 (Utilities|Struct|BreakS_AudioMapData (.Value (Utilities|Map|Find (Variables|Default|GetTimes%20to%20Sound%20Map) _keypin)))
              (LocalVariables|SetReturn (or (LocalVariables|GetReturn) (Utilities|Array|ContainsItem (Utilities|Struct|BreakS_AudioMapData (.Value (Utilities|Map|Find Map%20to%20Compare%20Against _valuepin))) _array_element_3))))))
        (:CompletedPin
          (return (LocalVariables|GetReturn))))
      (else
        (return false)))
    (else
      (return _output_get))))

(fn RemoveSound
  (bind _times_to_sound_map (Variables|Default|GetTimes%20to%20Sound%20Map))
  (bind _most_recent_time (Variables|Default|GetMost%20Recent%20Time))
  (bind (_value _returnvalue) (Utilities|Map|Find _times_to_sound_map _most_recent_time))
  (bind _soundsarray (Utilities|Struct|BreakS_AudioMapData _value))
  (if _returnvalue
    (Utilities|Array|RemoveIndex _soundsarray (- (Utilities|Array|Length _soundsarray) 1))))