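; Looper settings preset that derives its loop length from the sounds it holds.
; ComputeMaxLength walks every sound array in the sound map and keeps the longest duration found.
; That maximum becomes the preset's loop length and is logged with the class name.
; The running maximum is not reset inside the function, so it starts from its existing value.
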(fn ComputeMaxLength
  (bind _valuepin (Utilities|Map|ForEachLoop(Map) (Variables|Default|GetPSoundMap))
    (:then
      (for _array_element (Utilities|Struct|BreakS_AudioMapData _valuepin)
        (if (>= (Variables|/Script/Engine.SoundBase|GetDuration _array_element) (LocalVariables|GetCurrMaxLength))
          (LocalVariables|SetCurrMaxLength (Variables|/Script/Engine.SoundBase|GetDuration _array_element)))))
    (:CompletedPin
      (Variables|Default|SetPLoopLength (LocalVariables|GetCurrMaxLength))
      (Utilities|String|LogString (Utilities|String|Append (Utilities|GetClassDisplayName (Utilities|GetClass self)) ": Loop Length set to " (Utilities|String|ToString(Float) (LocalVariables|GetCurrMaxLength)))))))