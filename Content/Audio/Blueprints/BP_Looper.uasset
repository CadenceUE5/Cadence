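; Audio looper that replays a map of timestamped 2D sounds every loop, seeded with demo sounds when empty.
; A looping timer fires PerformLoop, which restarts the beat timer, broadcasts the loop dispatcher and starts playback; each beat also broadcasts a dispatcher.
; Playback sorts the timestamps and chains Delays through a recursive PlayNextSound event.
; AddSound records a sound at the current loop time, optionally rounded to the nearest beat.
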(event Custom|Perform%20Loop
  (Utilities|Time|SetTimerbyEvent (delegate Custom|Do%20Beat) (stale EventBeginPlay _output_get) true)
  (Default|CallEDDispatchLoop)
  (Variables|Default|SetBeats%20Completed 0)
  (CallFunction|PlayLoopSounds))

(event Custom|Do%20Beat
  (Default|CallEDDispatchBeat)
  (Math|Integer|IncrementInt (Variables|Default|GetBeats%20Completed)))

(event Custom|Play%20Loop%20Sounds
  (bind _keys (Utilities|Map|Keys (Variables|Default|GetTimes%20to%20Sound%20Map)))
  (bind _output_get (Variables|Default|SetTimes%20of%20Sounds _keys))
  (Class|KismetArrayLibrary|SortFloatArray _output_get)
  (Utilities|FlowControl|Delay (Utilities|Array|Get(acopy) (Variables|Default|GetTimes%20of%20Sounds)))
  (for _array_element (Utilities|Struct|BreakS_AudioMapData (.Value (Utilities|Map|Find (Variables|Default|GetTimes%20to%20Sound%20Map) (Utilities|Array|Get(acopy) (Variables|Default|GetTimes%20of%20Sounds)))))
    (Audio|PlaySound2D _array_element 1.0 1.0 0.0 0 0))
  (if (> (Utilities|Map|Length (Variables|Default|GetTimes%20to%20Sound%20Map)) 1)
    (CallFunction|PlayNextSound 1)
    (else
      (Development|PrintString "all sounds played"))))

(event Custom|Play%20Next%20Sound
  (params (Index :type Integer))
  (bind _times_of_sounds (Variables|Default|GetTimes%20of%20Sounds))
  (bind _output (Utilities|Array|Get(acopy) _times_of_sounds Index))
  (Utilities|FlowControl|Delay (- _output (Utilities|Array|Get(acopy) (Variables|Default|GetTimes%20of%20Sounds) (- Index 1))))
  (for _array_element (Utilities|Struct|BreakS_AudioMapData (.Value (Utilities|Map|Find (Variables|Default|GetTimes%20to%20Sound%20Map) _output)))
    (Audio|PlaySound2D _array_element 1.0 1.0 0.0 0 0))
  (if (== 0 (- (Utilities|Array|Length (Variables|Default|GetTimes%20of%20Sounds)) Index))
    (Development|PrintString "all sounds played")
    (else
      (CallFunction|PlayNextSound (+ Index 1)))))

(event EventBeginPlay
  (bind _output_get (Variables|Default|SetTime%20per%20Beat (Utilities|Operators|Divide (Variables|Default|GetLoop%20Length) (Variables|Default|GetBars%20per%20Loop) (Variables|Default|GetBeats%20per%20Bar))))
  (bind _returnvalue (Utilities|Time|SetTimerbyEvent (delegate Custom|Perform%20Loop) (Variables|Default|GetLoop%20Length) true))
  (Variables|Default|SetLoop%20Timer%20Handle _returnvalue)
  (if (Utilities|Map|IsEmpty (Variables|Default|GetTimes%20to%20Sound%20Map))
    (CallFunction|SetupDemoSounds)))

(fn ConstructionScript)

(fn SetupDemoSounds
  (bind _array (Utilities|Array|MakeArray "/Engine/EngineSounds/1kSineTonePing.1kSineTonePing" "/Engine/VREditor/Sounds/UI/Click_on_Button_Cue.Click_on_Button_Cue"))
  (bind _array_2 (Utilities|Array|MakeArray "/Engine/EngineSounds/1kSineTonePing.1kSineTonePing" "/Engine/VREditor/Sounds/UI/Camera_Shutter.Camera_Shutter"))
  (bind _times_to_sound_map (Variables|Default|GetTimes%20to%20Sound%20Map))
  (bind _s_audiomapdata (Utilities|Struct|MakeS_AudioMapData _array))
  (bind _s_audiomapdata_2 (Utilities|Struct|MakeS_AudioMapData _array_2))
  (Utilities|Map|Add _times_to_sound_map 0.25 _s_audiomapdata_2)
  (Utilities|Map|Add _times_to_sound_map 0.5 _s_audiomapdata)
  (Utilities|Map|Add _times_to_sound_map 1.0 _s_audiomapdata)
  (Utilities|Map|Add _times_to_sound_map 1.66 _s_audiomapdata_2))

(fn AddSound
  (params (Sound%20to%20Add :type Sound%20Base%20Object%20Reference))
  (bind _times_to_sound_map (Variables|Default|GetTimes%20to%20Sound%20Map))
  (bind _loop_timer_handle (Variables|Default|GetLoop%20Timer%20Handle))
  (bind _returnvalue (Class|KismetSystemLibrary|GetTimerElapsedTimeHandle _loop_timer_handle))
  (Utilities|FlowControl|Sequence
    (:then_0
      (if (Variables|Default|GetLock%20Added%20Sounds%20to%20Beat)
        (bind _output_get (LocalVariables|SetCurrent%20Time%20in%20Overall%20Loop (CallFunction|RoundTimetoNearestBeat (+ (* (Variables|Default|GetBeats%20Completed) (Variables|Default|GetTime%20per%20Beat)) _returnvalue) (/ (Variables|Default|GetLoop%20Length) (Variables|Default|GetBars%20per%20Loop)) (Variables|Default|GetBeats%20per%20Bar))))
        (else
          (LocalVariables|SetCurrent%20Time%20in%20Overall%20Loop _returnvalue))))
    (:then_1
      (if (.ReturnValue (Utilities|Map|Find _times_to_sound_map _output_get))
        (Utilities|Array|Add (Utilities|Struct|BreakS_AudioMapData (.Value (Utilities|Map|Find _times_to_sound_map _output_get))) Sound%20to%20Add)
        (else
          (Utilities|Map|Add _times_to_sound_map _output_get (Utilities|Struct|MakeS_AudioMapData (Utilities|Array|MakeArray Sound%20to%20Add))))))))