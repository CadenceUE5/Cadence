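; BP_Looper_Template is a template Blueprint for an audio looper, set up with demo sounds.
; SetupDemoSounds sets the loop length and fills TimesToSoundMap, keying SAudioMapData sound lists by time within the loop.
; Each entry pairs a sine-tone ping with a camera shutter or button click sound.
; The event graph is inert and the construction script only calls its parent, so this file contains no playback logic.
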(event EventBeginPlay
  (|CallParentFunction) ; This node is disabled and will not be called.\nDrag off pins to build functionality.
)

(event Collision|EventActorBeginOverlap
  (params (OtherActor :type Actor%20Object%20Reference)))

(event EventTick
  (params (DeltaSeconds :type Float%20%28single-precision%29)))

(fn ConstructionScript
  (|CallParentFunction))

(fn SetupDemoSounds
  (bind _array (Utilities|Array|MakeArray "/Engine/EngineSounds/1kSineTonePing.1kSineTonePing" "/Engine/VREditor/Sounds/UI/Click_on_Button_Cue.Click_on_Button_Cue"))
  (bind _array_2 (Utilities|Array|MakeArray "/Engine/EngineSounds/1kSineTonePing.1kSineTonePing" "/Engine/VREditor/Sounds/UI/Camera_Shutter.Camera_Shutter"))
  (bind _times_to_sound_map (Variables|Default|GetTimes%20to%20Sound%20Map))
  (bind _s_audiomapdata (Utilities|Struct|MakeS_AudioMapData _array))
  (bind _s_audiomapdata_2 (Utilities|Struct|MakeS_AudioMapData _array_2))
  (Variables|Default|SetLoop%20Length 4.0)
  (Utilities|Map|Add _times_to_sound_map 0.25 _s_audiomapdata_2)
  (Utilities|Map|Add _times_to_sound_map 0.5 _s_audiomapdata)
  (Utilities|Map|Add _times_to_sound_map 1.0 _s_audiomapdata)
  (Utilities|Map|Add _times_to_sound_map 1.66 _s_audiomapdata_2))