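; BP_LoopManager creates and controls the game's three audio loopers: User, Goal and Template.
; On BeginPlay, after a one-tick delay, it spawns them with a shared loop length from the template settings, with Goal muted and Template quieter.
; It loads goal sounds from class defaults, has the GameInstance acquire looper references, starts all loopers together, then fires an initialized dispatcher.
; Helper functions mute or unmute each looper by type.
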(event EventBeginPlay
  (bind _returnvalue (Math|Transform|MakeTransform "0, 0, 0"))
  (bind _template_settings (Variables|Default|GetTemplate%20Settings))
  (bind _plooplength (Variables|/Game/Audio/Blueprints/BP_LooperSettingsPreset.BP_LooperSettingsPreset_C|GetPLoopLength _template_settings))
  (Utilities|FlowControl|DelayUntilNextTick)
  (bind _returnvalue_2 (Game|SpawnActorfromClass "/Game/Audio/Blueprints/BP_Looper_User.BP_Looper_User_C" _returnvalue "Undefined" "MultiplyWithRoot" 0 0 _plooplength false 1.0 0))
  (Variables|Default|SetUser%20Looper _returnvalue_2)
  (bind _returnvalue_3 (Game|SpawnActorfromClass "/Game/Audio/Blueprints/BP_Looper_Goal.BP_Looper_Goal_C" _returnvalue "Undefined" "MultiplyWithRoot" 0 0 _plooplength true 1.0 0))
  (Variables|Default|SetGoal%20Looper _returnvalue_3)
  (bind _returnvalue_4 (Game|SpawnActorfromClass "/Game/Audio/Blueprints/BP_Looper_Template.BP_Looper_Template_C" _returnvalue "Undefined" "MultiplyWithRoot" 0 (Variables|Default|GetTemplate%20Settings) _plooplength false 0.2 0))
  (Variables|Default|SetTemplate%20Looper _returnvalue_4)
  (CallFunction|SetGoalSounds)
  (Class|BPIGameInstanceLooper|AcquireLooperReferences(Message) (Game|GetGameInstance))
  (CallFunction|StartAllLoopers)
  (Default|CallOnLoopersInitializedDispatcher))

(fn ConstructionScript)

(fn MuteLooper
  (params (Type%20to%20Mute :type E_LooperType%20Enum :default "NewEnumerator0"))
  (switch Utilities|FlowControl|Switch|SwitchonE_LooperType Type%20to%20Mute
    (:NewEnumerator0
      (Default|MuteSelf (Variables|Default|GetUser%20Looper)))
    (:NewEnumerator1
      (Default|MuteSelf (Variables|Default|GetGoal%20Looper)))
    (:NewEnumerator2
      (Default|MuteSelf (Variables|Default|GetTemplate%20Looper)))))

(fn UnmuteLooper
  (params (Type%20to%20Unmute :type E_LooperType%20Enum :default "NewEnumerator0"))
  (switch Utilities|FlowControl|Switch|SwitchonE_LooperType Type%20to%20Unmute
    (:NewEnumerator0
      (Default|UnmuteSelf (Variables|Default|GetUser%20Looper)))
    (:NewEnumerator1
      (Default|UnmuteSelf (Variables|Default|GetGoal%20Looper)))
    (:NewEnumerator2
      (Default|UnmuteSelf (Variables|Default|GetTemplate%20Looper)))))

(fn StartAllLoopers
  (Default|StartLoopOnce (Variables|Default|GetGoal%20Looper))
  (Default|StartLoopOnce (Variables|Default|GetUser%20Looper))
  (Default|StartLoopOnce (Variables|Default|GetTemplate%20Looper))
  (Development|PrintString "All Loopers started!"))

(fn SetGoalSounds
  (bind _bpgoalsound (Variables|Default|GetBPGoalSound))
  (bind _time_to_sound_map (Utilities|GetClassDefaults _bpgoalsound))
  (bind _goal_looper (Variables|Default|GetGoal%20Looper)
    (:then
      (Variables|/Game/Audio/Blueprints/BP_Looper_Base.BP_Looper_Base_C|SetTimes%20to%20Sound%20Map _goal_looper _time_to_sound_map))
    (:else
      (bind _goal_looper_2 (Class|BPIGameInstanceLooper|GetGoalLooper(Message) (Game|GetGameInstance)))
      (Variables|/Game/Audio/Blueprints/BP_Looper_Base.BP_Looper_Base_C|SetTimes%20to%20Sound%20Map _goal_looper_2 _time_to_sound_map)))
  (return))