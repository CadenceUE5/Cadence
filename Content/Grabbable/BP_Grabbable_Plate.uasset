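; BP_Grabbable_Plate is a grabbable VR plate that starts a gesture recorder and adds a sound when picked up.
; On grab, it finds the VRPawn and spawns a BP_GestureRecorder at a set offset along the headset's forward vector, scaled and rotated to align with the head's view.
; It then adds its Ding sound to the Looper.
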(event OnGrabbed(GrabComponent)
  (bind _returnvalue (Actor|GetActorOfClass "/Game/VRTemplate/Blueprints/VRPawn.VRPawn_C"))
  (Game|SpawnActorfromClass "/Game/Gesture/BP_GestureRecorder.BP_GestureRecorder_C" (Math|Transform|MakeTransform (+ (* (Math|Vector|GetForwardVector (Variables|/Game/VRTemplate/Blueprints/VRPawn.VRPawn_C|GetHeadMountedDisplayMesh _returnvalue)) (Variables|Default|GetOffset)) (.location (Transformation|GetWorldTransform (Variables|/Game/VRTemplate/Blueprints/VRPawn.VRPawn_C|GetHeadMountedDisplayMesh _returnvalue)))) (Class|KismetMathLibrary|MakeRotfromYX (Math|Vector|NegateVector (Math|Vector|GetForwardVector (Variables|/Game/VRTemplate/Blueprints/VRPawn.VRPawn_C|GetHeadMountedDisplayMesh _returnvalue))) (Math|Vector|GetRightVector (Variables|/Game/VRTemplate/Blueprints/VRPawn.VRPawn_C|GetHeadMountedDisplayMesh _returnvalue))) (Math|Conversions|ToVector(Float) (Variables|Default|GetScale))) "AlwaysSpawn" "OverrideRootScale" 0 0)
  (Default|AddSound (Variables|Default|GetLooper) "/Game/Audio/sound_effect/workshop/ding.ding"))

(event EventBeginPlay)

(event Collision|EventActorBeginOverlap
  (params (OtherActor :type Actor%20Object%20Reference)))

(event EventTick
  (params (DeltaSeconds :type Float%20%28single-precision%29)))

(fn ConstructionScript)