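; BP_Looper_Template is a looper Blueprint in CadenceCore that can take its times-to-sound map from a referenced LooperTemplate.
; On BeginPlay it runs CheckForTemplate, which overwrites its own TimesToSoundMap when the template is valid and its map is not empty.
; The copy happens before the parent BeginPlay call, so inherited startup logic sees the templated map.
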(event EventBeginPlay
  (CallFunction|CheckforTemplate)
  (|CallParentFunction))

(fn ConstructionScript
  (|CallParentFunction))

(fn CheckforTemplate
  (bind _looper_template (Variables|Default|GetLooper%20Template))
  (bind _times_to_sound_map (Variables|/Game/CadenceCore/Loop/Data/Template/BP_LoopTemplateData.BP_LoopTemplateData_C|GetTimes%20To%20Sound%20Map _looper_template))
  (Utilities|IsValid (Variables|Default|GetLooper%20Template)
    (:Is%20Valid
      (if (Utilities|Map|IsNotEmpty _times_to_sound_map)
        (Variables|Default|SetTimes%20to%20Sound%20Map _times_to_sound_map)))))