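; BP_BoomBox is a physical control with Compare, Switch, Undo and Clear buttons for the user's music loop.
; Collider overlaps call K8WorldSubsystem to score the user loop against the goal, toggle playback between them, undo or clear.
; Construction maps each button type to a dynamic material, whose ButtonEnabled parameter follows overlap begin and end.
; The Clear collider's begin overlap passes SWITCH, so clearing is never triggered.
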(event OnComponentEndOverlap(SwitchButtonCollider)
  (params (OverlappedComponent :type Primitive%20Component%20Object%20Reference) (OtherActor :type Actor%20Object%20Reference) (OtherComp :type Primitive%20Component%20Object%20Reference) (OtherBodyIndex :type Integer))
  ;[0.15 0.03753 0.08754 0.5] EndOverlaps
  (CallFunction|HandleBoomBoxButtonEndOverlap "NewEnumerator1"))

(event OnComponentBeginOverlap(SwitchButtonCollider)
  (params (OverlappedComponent :type Primitive%20Component%20Object%20Reference) (OtherActor :type Actor%20Object%20Reference) (OtherComp :type Primitive%20Component%20Object%20Reference) (OtherBodyIndex :type Integer) (bFromSweep :type Boolean) (SweepResult :type Hit%20Result%20Structure%20%28by%20ref%29))
  ;[0.05383 0.05003 0.15 0.5] BeginOverlaps
  (CallFunction|HandleBoomBoxButtonCallback "NewEnumerator1")
  (CallFunction|HandleBoomBoxButtonBeginOverlap "NewEnumerator1"))

(event OnComponentBeginOverlap(ClearButtonCollider)
  (params (OverlappedComponent :type Primitive%20Component%20Object%20Reference) (OtherActor :type Actor%20Object%20Reference) (OtherComp :type Primitive%20Component%20Object%20Reference) (OtherBodyIndex :type Integer) (bFromSweep :type Boolean) (SweepResult :type Hit%20Result%20Structure%20%28by%20ref%29))
  ;[0.05383 0.05003 0.15 0.5] BeginOverlaps
  (CallFunction|HandleBoomBoxButtonCallback "NewEnumerator1")
  (CallFunction|HandleBoomBoxButtonBeginOverlap "NewEnumerator1"))

(event OnComponentBeginOverlap(UndoButtonCollider)
  (params (OverlappedComponent :type Primitive%20Component%20Object%20Reference) (OtherActor :type Actor%20Object%20Reference) (OtherComp :type Primitive%20Component%20Object%20Reference) (OtherBodyIndex :type Integer) (bFromSweep :type Boolean) (SweepResult :type Hit%20Result%20Structure%20%28by%20ref%29))
  ;[0.05383 0.05003 0.15 0.5] BeginOverlaps
  (CallFunction|HandleBoomBoxButtonCallback "NewEnumerator2")
  (CallFunction|HandleBoomBoxButtonBeginOverlap "NewEnumerator2"))

(event OnComponentEndOverlap(UndoButtonCollider)
  (params (OverlappedComponent :type Primitive%20Component%20Object%20Reference) (OtherActor :type Actor%20Object%20Reference) (OtherComp :type Primitive%20Component%20Object%20Reference) (OtherBodyIndex :type Integer))
  ;[0.15 0.03753 0.08754 0.5] EndOverlaps
  (CallFunction|HandleBoomBoxButtonEndOverlap "NewEnumerator2"))

(event OnComponentBeginOverlap(CompareButtonCollider)
  (params (OverlappedComponent :type Primitive%20Component%20Object%20Reference) (OtherActor :type Actor%20Object%20Reference) (OtherComp :type Primitive%20Component%20Object%20Reference) (OtherBodyIndex :type Integer) (bFromSweep :type Boolean) (SweepResult :type Hit%20Result%20Structure%20%28by%20ref%29))
  ;[0.05383 0.05003 0.15 0.5] BeginOverlaps
  (CallFunction|HandleBoomBoxButtonCallback "NewEnumerator0")
  (CallFunction|HandleBoomBoxButtonBeginOverlap "NewEnumerator0"))

(event OnComponentEndOverlap(ClearButtonCollider)
  (params (OverlappedComponent :type Primitive%20Component%20Object%20Reference) (OtherActor :type Actor%20Object%20Reference) (OtherComp :type Primitive%20Component%20Object%20Reference) (OtherBodyIndex :type Integer))
  ;[0.15 0.03753 0.08754 0.5] EndOverlaps
  (CallFunction|HandleBoomBoxButtonEndOverlap "NewEnumerator3"))

(event OnComponentEndOverlap(CompareButtonCollider)
  (params (OverlappedComponent :type Primitive%20Component%20Object%20Reference) (OtherActor :type Actor%20Object%20Reference) (OtherComp :type Primitive%20Component%20Object%20Reference) (OtherBodyIndex :type Integer))
  ;[0.15 0.03753 0.08754 0.5] EndOverlaps
  (CallFunction|HandleBoomBoxButtonEndOverlap "NewEnumerator0"))

(fn ConstructionScript
  (bind _enumvalue (|ForEachEBoomBoxButtonType)
    (:LoopBody
      (Utilities|FlowControl|Sequence
        (:then_0
          (switch Utilities|FlowControl|Switch|SwitchonEBoomBoxButtonType _enumvalue
            (:NewEnumerator0
              (bind _returnvalue (Rendering|Material|CreateDynamicMaterialInstance "/Game/CadenceCore/Loop/BoomBoxMaterials/M_ButtonCompare.M_ButtonCompare" "None" "None" :!class /Script/Engine.KismetMaterialLibrary))
              (bind _output_get (LocalVariables|SetCreatedDynamicMaterialInstance _returnvalue))
              (Rendering|Material|SetMaterial (Variables|Default|GetCompareCylinder) 0 _output_get))
            (:NewEnumerator1
              (bind _returnvalue_2 (Rendering|Material|CreateDynamicMaterialInstance "/Game/CadenceCore/Loop/BoomBoxMaterials/M_ButtonSwitch.M_ButtonSwitch" "None" "None" :!class /Script/Engine.KismetMaterialLibrary))
              (bind _output_get_2 (LocalVariables|SetCreatedDynamicMaterialInstance _returnvalue_2))
              (Rendering|Material|SetMaterial (Variables|Default|GetSwitchCylinder) 0 _output_get_2))
            (:NewEnumerator2
              (bind _returnvalue_3 (Rendering|Material|CreateDynamicMaterialInstance "/Game/CadenceCore/Loop/BoomBoxMaterials/M_ButtonUndo.M_ButtonUndo" "None" "None" :!class /Script/Engine.KismetMaterialLibrary))
              (bind _output_get_3 (LocalVariables|SetCreatedDynamicMaterialInstance _returnvalue_3))
              (Rendering|Material|SetMaterial (Variables|Default|GetUndoCylinder) 0 _output_get_3))
            (:NewEnumerator3
              (bind _returnvalue_4 (Rendering|Material|CreateDynamicMaterialInstance "/Game/CadenceCore/Loop/BoomBoxMaterials/M_ButtonClear.M_ButtonClear" "None" "None" :!class /Script/Engine.KismetMaterialLibrary))
              (bind _output_get_4 (LocalVariables|SetCreatedDynamicMaterialInstance _returnvalue_4))
              (Rendering|Material|SetMaterial (Variables|Default|GetClearCylinder) 0 _output_get_4))))
        (:then_1
          (Utilities|Map|Add (Variables|Default|GetButtonTypeToMaterialInstanceMap) _enumvalue (LocalVariables|GetCreatedDynamicMaterialInstance)))))))

(fn HandleBoomBoxButtonCallback
  (params (Type :type EBoomBoxButtonType%20Enum :default "NewEnumerator0"))
  (bind _returnvalue (Subsystems|GetK8WorldSubsystem))
  (switch Utilities|FlowControl|Switch|SwitchonEBoomBoxButtonType Type
    (:NewEnumerator0
      (Variables|Default|SetComputedScore (Class|K8WorldSubsystem|ComputeUsertoGoalSimilarityScore _returnvalue)))
    (:NewEnumerator1
      (Class|K8WorldSubsystem|ToggleUserGoalLoopPlayback _returnvalue))
    (:NewEnumerator2
      (Class|K8WorldSubsystem|UndoLastIteminUserLoop _returnvalue))
    (:NewEnumerator3
      (Class|K8WorldSubsystem|ClearUserLoop _returnvalue))))

(fn HandleBoomBoxButtonEndOverlap
  (params (Type :type EBoomBoxButtonType%20Enum :default "NewEnumerator0"))
  (Rendering|Material|SetScalarParameterValue (.Value (Utilities|Map|Find (Variables|Default|GetButtonTypeToMaterialInstanceMap) Type)) "ButtonEnabled" 0.0 :!class /Script/Engine.MaterialInstanceDynamic))

(fn HandleBoomBoxButtonBeginOverlap
  (params (Type :type EBoomBoxButtonType%20Enum :default "NewEnumerator0"))
  (Rendering|Material|SetScalarParameterValue (.Value (Utilities|Map|Find (Variables|Default|GetButtonTypeToMaterialInstanceMap) Type)) "ButtonEnabled" 1.0 :!class /Script/Engine.MaterialInstanceDynamic))