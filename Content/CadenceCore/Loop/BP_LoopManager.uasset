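; Loop manager for a sound-looping game in which the player's User loop is checked against a Goal loop.
; On BeginPlay it spawns User, muted Goal and quieter Template loopers sharing the template sound's loop length, fills the goal sounds, notifies the GameInstance and starts all three.
; It toggles audibility between User and Goal, forwards sound edits to User, and broadcasts looper changes and tolerance-based validation results.
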(event EventBeginPlay
  (bind _returnvalue (Math|Transform|MakeTransform "0, 0, 0"))
  (bind _self self)
  (bind _templatesound (Variables|Default|GetTemplateSound))
  (bind _plooplength (Variables|/Game/CadenceCore/Loop/Data/Template/BP_LoopTemplate.BP_LoopTemplate_C|GetPLoopLength _templatesound))
  (bind _returnvalue_2 (Game|SpawnActorfromClass "/Game/CadenceCore/Loop/BP_Looper_User.BP_Looper_User_C" _returnvalue "Undefined" "MultiplyWithRoot" 0 0 _plooplength false 1.0 _self 0))
  (Variables|Default|SetUser%20Looper _returnvalue_2)
  (bind _returnvalue_3 (Game|SpawnActorfromClass "/Game/CadenceCore/Loop/BP_Looper_Goal.BP_Looper_Goal_C" _returnvalue "Undefined" "MultiplyWithRoot" 0 0 _plooplength true 1.0 _self 0))
  (Variables|Default|SetGoal%20Looper _returnvalue_3)
  (bind _returnvalue_4 (Game|SpawnActorfromClass "/Game/CadenceCore/Loop/BP_Looper_Template.BP_Looper_Template_C" _returnvalue "Undefined" "MultiplyWithRoot" 0 (Variables|Default|GetTemplateSound) _plooplength false 0.4 _self 0))
  (Variables|Default|SetTemplate%20Looper _returnvalue_4)
  (CallFunction|SetGoalSounds)
  (Class|BPIGlobalInstance|AcquireLoopManagerReference(Message) (Game|GetGameInstance))
  (CallFunction|StartAllLoopers)
  (Default|CallEDonLoopersInitialized))

(fn ConstructionScript)

(fn MuteLooper
  (params (Type%20to%20Mute :type E_LooperType%20Enum :default "NewEnumerator0"))
  (switch Utilities|FlowControl|Switch|SwitchonE_LooperType Type%20to%20Mute
    (:NewEnumerator0
      (Default|MuteSelf (Variables|Default|GetUser%20Looper))
      (Variables|Default|SetActiveLooper "NewEnumerator1"))
    (:NewEnumerator1
      (Default|MuteSelf (Variables|Default|GetGoal%20Looper))
      (Variables|Default|SetActiveLooper "NewEnumerator0"))
    (:NewEnumerator2
      (Default|MuteSelf (Variables|Default|GetTemplate%20Looper)))))

(fn UnmuteLooper
  (params (Type%20to%20Unmute :type E_LooperType%20Enum :default "NewEnumerator0"))
  (switch Utilities|FlowControl|Switch|SwitchonE_LooperType Type%20to%20Unmute
    (:NewEnumerator0
      (Default|UnmuteSelf (Variables|Default|GetUser%20Looper)))
    (:NewEnumerator1
      (Default|UnmuteSelf (Variables|Default|GetGoal%20Looper)))
    (:NewEnumerator2
      (Default|UnmuteSelf (Variables|Default|GetTemplate%20Looper)))))

(fn StartAllLoopers
  (Default|StartLoopOnce (Variables|Default|GetGoal%20Looper))
  (Default|StartLoopOnce (Variables|Default|GetUser%20Looper))
  (Default|StartLoopOnce (Variables|Default|GetTemplate%20Looper))
  (Development|PrintString "All Loopers started!"))

(fn SetGoalSounds
  (bind _bpgoalsound (Variables|Default|GetBPGoalSound))
  (bind _time_to_sound_map (Utilities|GetClassDefaults _bpgoalsound))
  (bind _goal_looper (Variables|Default|GetGoal%20Looper)
    (:then
      (Variables|/Game/CadenceCore/Loop/BP_Looper_Base.BP_Looper_Base_C|SetTimes%20to%20Sound%20Map _goal_looper _time_to_sound_map)
      (Variables|/Game/CadenceCore/Loop/BP_Looper_Base.BP_Looper_Base_C|SetTimes%20to%20Sound%20Map (Variables|Default|GetGoal%20Looper) _time_to_sound_map)
      (return))
    (:else)))

(fn ToggleActiveLooper
  (switch Utilities|FlowControl|Switch|SwitchonE_LooperType (Variables|Default|GetActiveLooper)
    (:NewEnumerator0
      (CallFunction|MuteLooper "NewEnumerator0")
      (CallFunction|UnmuteLooper "NewEnumerator1")
      (Default|CallEDonActiveLooperChanged "NewEnumerator1"))
    (:NewEnumerator1
      (CallFunction|MuteLooper "NewEnumerator1")
      (CallFunction|UnmuteLooper "NewEnumerator0")
      (Default|CallEDonActiveLooperChanged "NewEnumerator0"))
    (:NewEnumerator2
      (Development|PrintString "WARN: The template should never be the value of ActiveLooper."))))

(fn GetActiveLooper
  (return (Variables|Default|GetActiveLooper)))

(fn GetTemplateSound
  (return (Variables|Default|GetTemplateSound)))

(fn GetLoopLength
  (return (Variables|/Game/CadenceCore/Loop/Data/Template/BP_LoopTemplate.BP_LoopTemplate_C|GetPLoopLength (Variables|Default|GetTemplateSound))))

(fn GetLooperTimestoSoundMap
  (params (LooperType :type E_LooperType%20Enum :default "NewEnumerator0"))
  (bind _looperref (CallFunction|MaptoLooper LooperType))
  (return (Variables|/Game/CadenceCore/Loop/BP_Looper_Base.BP_Looper_Base_C|GetTimes%20to%20Sound%20Map _looperref)))

(fn MaptoLooper
  (params (Type :type E_LooperType%20Enum :default "NewEnumerator0"))
  (switch Utilities|FlowControl|Switch|SwitchonE_LooperType Type
    (:NewEnumerator0
      (return (Variables|Default|GetUser%20Looper)))
    (:NewEnumerator1
      (return (Variables|Default|GetGoal%20Looper)))
    (:NewEnumerator2
      (return (Variables|Default|GetTemplate%20Looper)))))

(fn ValidateUsertoGoalLooper
  (bind _validationtolerance (Variables|Default|GetValidationTolerance))
  (bind _maps_equivalent (Default|ValidateTolerance (Variables|Default|GetUser%20Looper) (Variables|/Game/CadenceCore/Loop/BP_Looper_Base.BP_Looper_Base_C|GetTimes%20to%20Sound%20Map (Variables|Default|GetGoal%20Looper)) _validationtolerance))
  (Default|CallEDonValidateLoopers _maps_equivalent _validationtolerance))

(fn ClearUserLooperSounds
  (Default|ClearAllSounds (Variables|Default|GetUser%20Looper)))

(fn AddSoundtoUserLooper
  (params (SoundToAdd :type Sound%20Base%20Object%20Reference) (Context :type Grabbable%20Material%20Pair%20Structure))
  (Default|AddSound (Variables|Default|GetUser%20Looper) SoundToAdd Context))