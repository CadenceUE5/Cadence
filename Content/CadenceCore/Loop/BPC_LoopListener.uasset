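; BPC_LoopListener is a component that relays events from Cadence's global loop manager to its own event dispatchers.
; On BeginPlay it waits for the game instance's manager-acquired event, caches the manager, binds to its looper events and announces that the listener is ready.
; Forwarders re-broadcast looper initialization, active looper change, validation, global loop and sound-added events, but the sounds-cleared forwarder calls itself instead of a dispatcher.
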(event Custom|BindAll
  (Utilities|FlowControl|Sequence
    (:then_0
      (bind _loop_manager (Default|GetGlobalLoopManager (stale EventBeginPlay _asgi_cadence)))
      (bind _output_get (Variables|Default|SetLoopManagerRef _loop_manager)))
    (:then_1
      (EventDispatchers|BindEventtoEDonLoopersInitialized _output_get (EventDispatchers|CreateEvent :!event Custom|ForwardOnLoopersInitialized))
      (EventDispatchers|BindEventtoEDonActiveLooperChanged _output_get (EventDispatchers|CreateEvent :!event Custom|ForwardOnActiveLooperChanged))
      (EventDispatchers|BindEventtoEDonValidateLoopers _output_get (EventDispatchers|CreateEvent :!event Custom|ForwardOnValidateLoopers))
      (EventDispatchers|BindEventtoEDGlobalonDoLoop _output_get (EventDispatchers|CreateEvent :!event Custom|ForwardOnGlobalDoLoop))
      (EventDispatchers|BindEventtoEDUseronAddSound _output_get (EventDispatchers|CreateEvent :!event Custom|ForwardOnUserLooperAddSound))
      (EventDispatchers|BindEventtoEDUseronSoundsCleared _output_get (EventDispatchers|CreateEvent :!event Custom|ForwardOnUserLooperClearSounds)))
    (:then_2
      (Default|CallOnListenerComponentReady))))

(event Custom|ForwardOnLoopersInitialized
  (Default|CallOnLoopersInitialized))

(event Custom|ForwardOnActiveLooperChanged
  (params (NewLooperType :type E_LooperType%20Enum :default "NewEnumerator0"))
  (Default|CallOnActiveLooperChanged NewLooperType))

(event Custom|ForwardOnValidateLoopers
  (params (Result :type Boolean) (ValidationTolerance :type Float%20%28double-precision%29))
  (Default|CallOnValidateLoopers Result ValidationTolerance))

(event Custom|ForwardOnGlobalDoLoop
  (Default|CallOnGlobalDoLoop))

(event Custom|ForwardOnUserLooperAddSound
  (params (Sound%20Added :type Sound%20Base%20Object%20Reference) (Time%20Added%20In%20Loop :type Float%20%28double-precision%29))
  (Default|CallOnUserLooperAddSound Sound%20Added Time%20Added%20In%20Loop))

(event Custom|ForwardOnUserLooperClearSounds
  (CallFunction|ForwardonUserLooperClearSounds))

(event EventBeginPlay
  (bind _asgi_cadence (Utilities|Casting|CastToGI_Cadence (Game|GetGameInstance)))
  (EventDispatchers|BindEventtoEDGlobalLoopManagerAcquired _asgi_cadence (delegate Custom|BindAll)))

(fn GetLoopManagerRef
  (return (Variables|Default|GetLoopManagerRef)))