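; Grabbable actor that turns collisions with other grabbables into sound loop items added to the user's loop.
; A DataAsset supplies its mesh and material type; each material pair looks up a table row for sound and overlay color.
; Impulse strength sets volume, a GUID comparison lets only one actor register each hit, and a gate with delay throttles detection.
; World settings supply sensitivity, throttle interval and table.
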(event EventBeginPlay
  (bind _returnvalue (Subsystems|GetK8WorldSubsystem))
  (bind _settings (Variables|/Script/Cadence.K8_WorldSubsystem|GetSettings _returnvalue))
  ;[0.03355 0.03608 0.15 0.5] Get configurable properties from world settings
  (CallFunction|Initialize)
  (Variables|Default|SetImpulseSensivity (Variables|/Script/Cadence.K8WorldSubsystemSettings|GetGrabbableImpulseSensitivity _settings))
  (Variables|Default|SetHitDetectionFrequency (Variables|/Script/Cadence.K8WorldSubsystemSettings|GetGrabbableHitDetectionFrequency _settings))
  (bind _grabbablematerialdatatable (Variables|/Script/Cadence.K8WorldSubsystemSettings|GetGrabbableMaterialDataTable _settings)
    (:then
      (Variables|Default|SetDataTableAsset _grabbablematerialdatatable))
    (:else)))

(event Collision|EventHit
  (params (MyComp :type Primitive%20Component%20Object%20Reference) (Other :type Actor%20Object%20Reference) (OtherComp :type Primitive%20Component%20Object%20Reference) (bSelfMoved :type Boolean) (HitLocation :type Vector :default "0, 0, 0") (HitNormal :type Vector :default "0, 0, 0") (NormalImpulse :type Vector :default "0, 0, 0") (Hit :type Hit%20Result%20Structure%20%28by%20ref%29))
  ;[0.15 0.05221 0.146 0.5] Event Hit
  (bind (_shouldregisterhit _rowname _grabbablematerialpairdata) (CallFunction|HandleHit Other))
  (if _shouldregisterhit
    (Utilities|FilterHitDetectionFrequency
      (:Exit
        (bind _loopitem (CallFunction|ConvertGrabbableMaterialPairtoLoopItem _grabbablematerialpairdata (CallFunction|MapVectorMagnitudetoStrength01 (Math|Vector|VectorLength NormalImpulse) (Variables|Default|GetImpulseSensivity)) (Transformation|GetWorldLocation (Variables|Default|GetStaticMesh)) _rowname))
        (Class|K8WorldSubsystem|AddItemtoUserLoop (Subsystems|GetK8WorldSubsystem) _loopitem)))))

(fn ConstructionScript
  (CallFunction|Initialize))

(fn FindDataTableRowforGrabbables
  (params (GrabbableA :type BP%20Grabbable%20Actor%20Object%20Reference) (GrabbableB :type BP%20Grabbable%20Actor%20Object%20Reference) (DataTable :type Data%20Table%20Object%20Reference))
  (bind _dataasset (Variables|Default|GetDataAsset)
    (:then
      (bind _dataasset_2 (Variables|BP_Grabbable_Actor_C|GetDataAsset GrabbableB)
        (:then
          (bind _returnvalue (Utilities|GetDataTableRow DataTable (Class|GrabbableFunctionLibrary|MakeGrabbableMaterialPairRowName (Variables|/Script/Cadence.GrabbablePrimaryDataAsset|GetMaterialType _dataasset) (Variables|/Script/Cadence.GrabbablePrimaryDataAsset|GetMaterialType _dataasset_2)))
            (:then
              (return true (Class|GrabbableFunctionLibrary|MakeGrabbableMaterialPairRowName (Variables|/Script/Cadence.GrabbablePrimaryDataAsset|GetMaterialType _dataasset) (Variables|/Script/Cadence.GrabbablePrimaryDataAsset|GetMaterialType _dataasset_2)) _returnvalue))
            (:RowNotFound
              (return false (Class|GrabbableFunctionLibrary|MakeGrabbableMaterialPairRowName (Variables|/Script/Cadence.GrabbablePrimaryDataAsset|GetMaterialType _dataasset) (Variables|/Script/Cadence.GrabbablePrimaryDataAsset|GetMaterialType _dataasset_2)) ""))))
        (:else)))
    (:else)))

(fn MapVectorMagnitudetoStrength01
  (params (Magnitude :type Float%20%28double-precision%29) (Sensitivity :type Float%20%28double-precision%29))
  (return (Math|Float|Clamp(Float) (/ Magnitude Sensitivity))))

(fn ConvertGrabbableMaterialPairtoLoopItem
  (params (GrabbableMaterialPair :type Grabbable%20Material%20Pair%20Structure%20%28by%20ref%29) (VolumeMultiplier :type Float%20%28single-precision%29) (WorldPosition :type Vector) (Instigator%20Name :type Name))
  (bind (_materiala _materialb _sound _color) (Utilities|Struct|BreakGrabbableMaterialPair GrabbableMaterialPair))
  (return (Utilities|Struct|MakeLoopItem "" _sound _color VolumeMultiplier WorldPosition "SPATIAL" Instigator%20Name)))

(fn HandleHit
  (params (HitActor :type Actor%20Object%20Reference))
  (bind _asbp_grabbable_actor (Utilities|Casting|CastToBP_Grabbable_Actor HitActor))
  (bind (_found _rowname _grabbablematerialpairdata) (CallFunction|FindDataTableRowforGrabbables self _asbp_grabbable_actor (Variables|Default|GetDataTableAsset)))
  (if _found
    (CallFunction|SetOverlayColorfromGrabbableMaterialPair _grabbablematerialpairdata)
    (bind _hasgreaterguid (CallFunction|CompareActorsbyGuid HitActor self))
    (return _hasgreaterguid _rowname _grabbablematerialpairdata)))

(fn CompareActorsbyGuid
  (params (ActorA :type Actor%20Object%20Reference) (ActorB :type Actor%20Object%20Reference))
  (return (Class|GrabbableFunctionLibrary|IsGuidGreaterThan (Variables|/Script/Engine.Actor|GetActorGuid ActorA) (Variables|Default|GetActorGuid ActorB))))

(fn SetOverlayColorfromGrabbableMaterialPair
  (params (GrabbableMaterialPair :type Grabbable%20Material%20Pair%20Structure%20%28by%20ref%29))
  (Rendering|Material|SetVectorParameterValue (Variables|Default|GetMI_Overlay) "BaseColor" (Math|Conversions|ToLinearColor(Color) (.Color (Utilities|Struct|BreakGrabbableMaterialPair GrabbableMaterialPair))) :!class /Script/Engine.MaterialInstanceDynamic))

(fn Initialize
  (bind _dataasset (Variables|Default|GetDataAsset)
    (:then
      (Components|StaticMesh|SetStaticMesh (Variables|Default|GetStaticMesh) (Variables|/Script/Cadence.GrabbablePrimaryDataAsset|GetMesh _dataasset))
      (bind _returnvalue (Rendering|Material|CreateDynamicMaterialInstance "/Game/CadenceCore/Grabbable/M_GrabbableOverlay_Base.M_GrabbableOverlay_Base" "None" "None" :!class /Script/Engine.KismetMaterialLibrary))
      (bind _output_get (Variables|Default|SetMI_Overlay _returnvalue))
      (Rendering|Material|SetOverlayMaterial (Variables|Default|GetStaticMesh) _output_get :!class /Script/Engine.MeshComponent))
    (:else)))